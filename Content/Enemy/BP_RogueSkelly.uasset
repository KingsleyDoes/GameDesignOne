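; BP_RogueSkelly is the Rogue skeleton enemy, tagging itself with Rogue on BeginPlay.
; Idle, RangedAttack, BarrageAttack and Die events set numeric Action and State values, which look like animation drivers.
; Both attacks switch Action between two phases using fixed delays, then return to Idle.
; Die randomizes Action within a range, sets the death State and adds the Status.Dead tag.
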(event `Idle`
  (set `self.Action` 0.0)
  (set `self.State` 0.0))

(event `self.ReceiveBeginPlay`
  (bind _tagcontainer (`self.GetGameplayTagContainer`))
  (bind _output_get (set `self.Tag Container` _tagcontainer))
  (`BlueprintGameplayTagLibrary.AddGameplayTag` _output_get (`self.Rogue`)))

(event `Ranged Attack`
  (set `self.Action` 25.0)
  (set `self.State` 25.0)
  (`KismetSystemLibrary.Delay` 1.0)
  (set `self.Action` 75.0)
  (`KismetSystemLibrary.Delay` 1.1)
  (`self.Idle`))

(event `Die`
  (set `self.Action` (`KismetMathLibrary.RandomFloatInRange` 50.0 100.0))
  (set `self.State` 100.0)
  (`BlueprintGameplayTagLibrary.AddGameplayTag` (stale `self.ReceiveBeginPlay` _output_get) (struct :`TagName` "Status.Dead")))

(event `Barrage Attack`
  (set `self.Action` 50.0)
  (set `self.State` 25.0)
  (`KismetSystemLibrary.Delay` 1.2)
  (set `self.Action` 75.0)
  (`KismetSystemLibrary.Delay` 1.1)
  (`self.Idle`))

(fn `GetGameplayTagContainer`
  (returns (TagContainer :type "GameplayTagContainer Structure"))
  (return))

(fn `UserConstructionScript`)