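; BP_Projectile is a projectile actor that delivers a battle unit's attack damage on impact.
; On BeginPlay its sphere ignores the instigator during movement.
; On hit it spawns an impact effect, then applies damage calculated by the instigator's combat component to that component's stored target, regardless of the actor struck.
; It destroys itself after a short delay, only if the instigator is a BP_UnitBase.
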(event `self.ReceiveBeginPlay`
  (`PrimitiveComponent.IgnoreActorWhenMoving` (`self.Sphere`) (`self.GetInstigator`) true))

(event `self.ReceiveHit`
  (params (MyComp :type "PrimitiveComponent Object Reference") (Other :type "Actor Object Reference") (OtherComp :type "PrimitiveComponent Object Reference") (bSelfMoved :type Boolean) (HitLocation :type "Vector Structure") (HitNormal :type "Vector Structure") (NormalImpulse :type "Vector Structure") (Hit :type "HitResult Structure (by ref)"))
  (`GameplayStatics.SpawnEmitterAtLocation` (`self.ImpactEffect`))
  (bind _asbp_unit_base (cast `/Game/BattleTutorial/BP_UnitBase` (`self.GetInstigator`)))
  (bind _ac_combatcomponent (`/Game/BattleTutorial/BP_UnitBase.AC_CombatComponent` _asbp_unit_base))
  (bind _basedam (`/Game/BattleTutorial/AC_CombatComponent.CalculateDamage` _ac_combatcomponent))
  (`GameplayStatics.ApplyDamage` (`/Game/BattleTutorial/AC_CombatComponent.UnitTarget` _ac_combatcomponent) _basedam null _asbp_unit_base (`self.Damage Type Class`))
  (`KismetSystemLibrary.Delay` 1.0)
  (`self.K2_DestroyActor`))

(fn `UserConstructionScript`)