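; Battle game mode that sets up the tutorial battle's camera, party and enemy lists, and runs its turn queue.
; On BeginPlay it blends to the main battle camera, gathers units, then after a short delay adds party members to the player controller's battle HUD.
; Units queue through TurnRequest, and a DoOnce gate starts one turn at a time via the combat component, binding its turn-ended event.
; ReadyNextTurn reopens the gate and starts any queued turn.
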(event `self.ReceiveBeginPlay`
  (bind _returnvalue (`GameplayStatics.GetActorOfClass` "/Game/BattleTutorial/BP_BattleCam_Main.BP_BattleCam_Main_C"))
  (bind _output_get (set `self.MainCam` _returnvalue))
  (`PlayerController.SetViewTargetWithBlend` (`GameplayStatics.GetPlayerController` 0) _output_get 0.0 "VTBlend_Linear" 0.0 false)
  (bind _outactors (`GameplayStatics.GetAllActorsOfClass` "/Game/BattleTutorial/CBP_PartyUnitBase.CBP_PartyUnitBase_C"))
  (set `self.PartyMembers` _outactors)
  (bind _outactors_2 (`GameplayStatics.GetAllActorsOfClass` "/Game/BattleTutorial/CBP_EnemyUnitBase.CBP_EnemyUnitBase_C"))
  (set `self.EnemyPartyMembers` _outactors_2)
  (`KismetSystemLibrary.Delay` 0.2)
  (bind _asbp_battle_player_controller (cast `/Game/BattleTutorial/BP_BattlePlayerController` (`GameplayStatics.GetPlayerController` 0)))
  (set `self.GM Battle HUD` (`/Game/BattleTutorial/BP_BattlePlayerController.BattleHUD` _asbp_battle_player_controller))
  (for _array_element (`self.PartyMembers`)
    (`/Game/Widgets/TutorialWidgets/W_BattleHUD.AddPartyUnitToHUD` (`self.GM Battle HUD`) _array_element)))

(event `TurnRequest`
  (params (Unit :type "/Game/BattleTutorial/BP_UnitBase Object Reference"))
  (`KismetArrayLibrary.Array_AddUnique` (`self.TurnOrder`) Unit)
  (`self.StartTurn`))

(event `StartTurn`
  (bind _ac_combatcomponent (`/Game/BattleTutorial/BP_UnitBase.AC_CombatComponent` (`|GetArrayItem` (`self.TurnOrder`))))
  (`/Engine/EditorBlueprintResources/StandardMacros.DoOnce` false :!label _label
    (:`Completed`
      (if (`KismetArrayLibrary.Array_IsValidIndex` (`self.TurnOrder`))
        (`/Game/BattleTutorial/AC_CombatComponent.StartUnitTurn` _ac_combatcomponent)
        (add `/Game/BattleTutorial/AC_CombatComponent.TurnEnded` _ac_combatcomponent (`|CreateDelegate` :!event `ReadyNextTurn`))
        (`KismetArrayLibrary.Array_Remove` (`self.TurnOrder`))
        (else
          (`self.ReadyNextTurn`))))))

(event `ReadyNextTurn`
  (`|ExecutionSequence`
    (:`then_0`
      (goto _label :!via `Reset`))
    (:`then_1`
      (if (`KismetArrayLibrary.Array_IsValidIndex` (`self.TurnOrder`))
        (`self.StartTurn`)))))

(fn `UserConstructionScript`)