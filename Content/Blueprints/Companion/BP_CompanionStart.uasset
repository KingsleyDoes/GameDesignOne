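; BP_CompanionStart is a placeholder for the ranger companion, lying in an idle loop until the player first reaches it.
; When BP_TopDownCharacter overlaps ImmobilityBox, the box is destroyed and a W_Text subtitle widget shows the first DT_SubCompanion1 line.
; It then plays the stand-up animation and, after a short delay, spawns BP_Companion at a hard-coded location and destroys itself.
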(event `self.ReceiveBeginPlay`
  (bind _tagcontainer (`self.GetGameplayTagContainer`))
  (bind _output_get (set `self.Tag Container` _tagcontainer))
  (`BlueprintGameplayTagLibrary.AddGameplayTag` _output_get (struct :`TagName` "Characters.Ranger"))
  (set `self.Immobile` true)
  (`self.NotYetMet`))

(event `NotYetMet`
  (`SkeletalMeshComponent.PlayAnimation` (`self.Mesh`) "/Game/Blueprints/Companion/Rogue/RogueNoProps_Anim_Rig_Rig_Lie_Idle.RogueNoProps_Anim_Rig_Rig_Lie_Idle" (`self.Immobile`)))

(event `Mobilized`
  (if (not (`self.Immobile`))
    (`SkeletalMeshComponent.PlayAnimation` (`self.Mesh`) "/Game/Blueprints/Companion/Rogue/RogueNoProps_Anim_Rig_Rig_Lie_StandUp.RogueNoProps_Anim_Rig_Rig_Lie_StandUp" false)
    (`KismetSystemLibrary.Delay` 2.0)
    (`self.EnableInput` (`GameplayStatics.GetPlayerController` 0))
    (`|SpawnActorFromClass` "/Game/Blueprints/Companion/BP_Companion.BP_Companion_C" (`KismetMathLibrary.MakeTransform` (-10325.319973 2966.357657 133.875697)) "Undefined" "MultiplyWithRoot" null null null)
    (`self.K2_DestroyActor`)))

(event `self.Immobility Box.OnComponentBeginOverlap`
  (params (OverlappedComponent :type "PrimitiveComponent Object Reference") (OtherActor :type "Actor Object Reference") (OtherComp :type "PrimitiveComponent Object Reference") (OtherBodyIndex :type Integer) (bFromSweep :type Boolean) (SweepResult :type "HitResult Structure (by ref)"))
  (if true
    (cast `/Game/TopDown/Blueprints/BP_TopDownCharacter` OtherActor)
    (`ActorComponent.K2_DestroyComponent` (`self.Immobility Box`))
    (set `self.Immobile` false)
    (bind _returnvalue (`|CreateWidget` "/Game/Widgets/Subtitles/W_Text.W_Text_C" null (make `DataTableRowHandle` "/Game/Widgets/Subtitles/DT_SubCompanion1.DT_SubCompanion1" "1")))
    (`UserWidget.AddToViewport` _returnvalue 0)
    (`self.Mobilized`)))

(fn `GetGameplayTagContainer`
  (returns (TagContainer :type "GameplayTagContainer Structure"))
  (return))

(fn `UserConstructionScript`)