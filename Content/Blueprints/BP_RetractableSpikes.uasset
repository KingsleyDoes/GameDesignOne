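; BP_RetractableSpikes is a spike trap that slides its Spikes component from an extended to a retracted position.
; The Retract timeline lerps between the relative locations of the Out and Retracted components, with a 2D sound cue played at the start.
; It runs on BeginPlay and again when a BP_TopDownCharacter with HasTrapKit overlaps the Box.
; Every Box overlap also prints a debug string, and no damage logic is present.
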(event `self.ReceiveBeginPlay`
  (`GameplayStatics.PlaySound2D` "/Game/audio/dungeonSpecific/retract_cue.retract_cue" 1.0 1.0 0.0 null null :!label _label)
  (bind (_direction _newtrack_0) (`Timeline|Retract`)
    (:`Update`
      (`SceneComponent.K2_SetRelativeLocation` (`self.Spikes`) (`KismetMathLibrary.VLerp` (`SceneComponent.RelativeLocation` (`self.Out`)) (`SceneComponent.RelativeLocation` (`self.Retracted`)) _newtrack_0) false false))))

(event `self.Box.OnComponentBeginOverlap`
  (params (OverlappedComponent :type "PrimitiveComponent Object Reference") (OtherActor :type "Actor Object Reference") (OtherComp :type "PrimitiveComponent Object Reference") (OtherBodyIndex :type Integer) (bFromSweep :type Boolean) (SweepResult :type "HitResult Structure (by ref)"))
  (`KismetSystemLibrary.PrintString` "Hello")
  (bind _asbp_top_down_character (cast `/Game/TopDown/Blueprints/BP_TopDownCharacter` OtherActor))
  (if (`/Game/TopDown/Blueprints/BP_TopDownCharacter.HasTrapKit` _asbp_top_down_character)
    (goto _label)))

(fn `UserConstructionScript`)