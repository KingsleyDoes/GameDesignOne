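; Villager AI character that wanders between village patrol points and can spot the player when hostile.
; On BeginPlay it shuffles the tagged patrol points, randomizes walk speed, then loops through them with AIMoveTo and a pause, reshuffling each cycle.
; An FOV overlap with the top-down character shows a subtitle, raises speed and calls Chase, which is empty because its follow-player logic is disconnected.
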(event `self.ReceiveBeginPlay`
  (bind _tagcontainer (`self.GetGameplayTagContainer`))
  (set `self.Tag Container` _tagcontainer)
  (bind _outactors (`GameplayStatics.GetAllActorsOfClassWithTag` "/Game/Blueprints/villagers/BP_VillagePatrolPoint.BP_VillagePatrolPoint_C" "PatrolPoint.Village"))
  (bind _output_get (set `self.PatrolPoints` _outactors))
  (`KismetArrayLibrary.Array_Shuffle` _output_get)
  (set `self.PatrolPointLength` (`KismetArrayLibrary.Array_Length` _output_get))
  (set `CharacterMovementComponent.MaxWalkSpeed` (`KismetMathLibrary.Conv_IntToDouble` (* (`KismetMathLibrary.RandomIntegerInRange` 5 12) 25)) (`self.CharacterMovement`))
  (`self.GoPatrol`))

(event `Chase`
  ;[1 0.4011 0.4442] Chase Player
)

(event `GoPatrol`
  ;[0.808 1 0.5363] Patrol as normal
  (`|AIMoveTo` self (`self.K2_GetActorLocation` (`|GetArrayItem` (`self.PatrolPoints`) (`self.CurrentPatrolPoint`))) null 200.0
    (:`OnSuccess`
      _)
    (:`OnFail`
      _))
  (bind _result (`/Engine/EditorBlueprintResources/StandardMacros.IncrementInt` (`self.CurrentPatrolPoint`))
    (:`  `
      (if (>= _result (`self.PatrolPointLength`))
        (set `self.CurrentPatrolPoint` 0)
        (`KismetArrayLibrary.Array_Shuffle` (`self.PatrolPoints`)))
      (`KismetSystemLibrary.Delay` 5.0)
      (`self.GoPatrol`))))

(event `self.FOV.OnComponentBeginOverlap`
  (params (OverlappedComponent :type "PrimitiveComponent Object Reference") (OtherActor :type "Actor Object Reference") (OtherComp :type "PrimitiveComponent Object Reference") (OtherBodyIndex :type Integer) (bFromSweep :type Boolean) (SweepResult :type "HitResult Structure (by ref)"))
  ;[0.3134 0.6485 1] See Player
  (if (`self.Hostile`)
    (bind _asbp_top_down_character (cast `/Game/TopDown/Blueprints/BP_TopDownCharacter` OtherActor))
    (set `self.As BP Top Down Character` _asbp_top_down_character)
    (`self.SpotPlayer`)))

(event `SpotPlayer`
  ;[0.3134 0.6485 1] See Player
  (bind _returnvalue (`|CreateWidget` "/Game/Widgets/Subtitles/W_Text.W_Text_C" null (make `DataTableRowHandle` "/Game/Widgets/Subtitles/DT_SubPatroller.DT_SubPatroller" "1")))
  (`UserWidget.AddToViewport` _returnvalue 0)
  (`KismetSystemLibrary.Delay` 0.5)
  (set `CharacterMovementComponent.MaxWalkSpeed` 450.0 (`self.CharacterMovement`))
  (`self.Chase`))

(fn `GetGameplayTagContainer`
  (returns (TagContainer :type "GameplayTagContainer Structure"))
  (return))

(fn `UserConstructionScript`)