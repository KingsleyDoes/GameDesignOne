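; BP_EnemySpawnManager spawns enemies at level spawners and ends the battle when its enemy count runs out.
; On BeginPlay it gathers every BP_EnemySpawner and spawns at each one's transform, though the spawn call shows no class.
; RemoveEnemyAndCheck decrements the count and, at zero or below, sets EnemiesDefeated and spawns BP_EndBattle rather than another wave.
; The logic assigning Manager and incrementing the count is disconnected.
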(event `self.ReceiveBeginPlay`
  (bind _outactors (`GameplayStatics.GetAllActorsOfClass` "/Game/Blueprints/Enemies/BP_EnemySpawner.BP_EnemySpawner_C"))
  (set `self.Spawners` _outactors)
  (`self.Spawn Enemies`))

(event `Spawn Enemies`
  (for _array_element (`self.Spawners`)
    (bind (_returnvalue_location _returnvalue_rotation) (`KismetMathLibrary.BreakTransform` (`SceneComponent.K2_GetComponentToWorld` (`/Game/Blueprints/Enemies/BP_EnemySpawner.DefaultSceneRoot` _array_element))))
    (`|SpawnActorFromClass` "/Game/Enemy/BP_RogueSkelly.BP_RogueSkelly_C" (`KismetMathLibrary.MakeTransform` _returnvalue_location _returnvalue_rotation) "Undefined" "MultiplyWithRoot" null null) ; Create a new enemy at the spawner's location and rotation.
  ))

(event `RemoveEnemyAndCheck`
  (`/Engine/EditorBlueprintResources/StandardMacros.DecrementInt` (`self.CurrentEnemyTotal`)
    (:`  `
      (if (not (> (`self.CurrentEnemyTotal`) 0))
        (set `self.EnemiesDefeated` true)
        (`|SpawnActorFromClass` "/Game/Blueprints/BP_EndBattle.BP_EndBattle_C" (`KismetMathLibrary.Conv_VectorToTransform` (`SceneComponent.RelativeLocation` (`self.DefaultSceneRoot`))) "Undefined" "MultiplyWithRoot" null null)))))

(fn `UserConstructionScript`)